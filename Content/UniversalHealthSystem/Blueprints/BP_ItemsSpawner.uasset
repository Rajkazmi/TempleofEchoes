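; Item spawner that shows a countdown, then spawns a random item class just above itself with randomized stat count.
; The authority runs a looping one-second timer, clears it on spawn and restarts it when the item is destroyed.
; The countdown replicates through a RepNotify text variable, with Server and Multi events toggling its visibility.
; Tick turns the text's yaw toward the local player camera.
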(event `self.ReceiveBeginPlay`
  (`KismetSystemLibrary.Delay` 1.0)
  (`/Engine/EditorBlueprintResources/ActorMacros.Switch Has Authority`
    (:`Authority`
      (bind _output_get (set `self.Timer` (`self.SpawnTime`)))
      (set `self.Name` (`KismetTextLibrary.Conv_IntToText` _output_get false false))
      (`self.-StartTimerToRespawnItem`))))

(event `self.ReceiveTick`
  (params (DeltaSeconds :type "Float (single-precision)"))
  (bind _returnvalue (`GameplayStatics.GetPlayerCameraManager` 0))
  ;[1 1 1] Rotation to Camera
  (`/Engine/EditorBlueprintResources/StandardMacros.IsValid` _returnvalue
    (:`Is Valid`
      (`SceneComponent.K2_SetWorldRotation` (`self.TextRender`) (`KismetMathLibrary.MakeRotator` 0.0 0.0 (+ (.yaw (`KismetMathLibrary.FindLookAtRotation` (`self.K2_GetActorLocation` _returnvalue) (`self.K2_GetActorLocation`))) 180.0)) false false))))

(event `-RespawnStart`
  (params (DestroyedActor :type "Actor Object Reference"))
  (set `self.Spawned` false)
  (`self.-StartTimerToRespawnItem`))

(event `-HiddenText_Multi`
  (params (NewHidden :type Boolean))
  (`SceneComponent.SetHiddenInGame` (`self.TextRender`) NewHidden false))

(event `-HiddenText_Server`
  (params (NewHidden :type Boolean))
  (`self.-HiddenText_Multi` NewHidden))

(fn `-SpawnItem`
  (bind _itemsclassforspawn (`self.ItemsClassForSpawn`))
  (bind _returnvalue (`|SpawnActorFromClass` (`|GetArrayItem` _itemsclassforspawn (`KismetMathLibrary.RandomIntegerInRange` 0 (`KismetArrayLibrary.Array_LastIndex` _itemsclassforspawn))) (`KismetMathLibrary.MakeTransform` (`KismetMathLibrary.MakeVector` (.x (`self.K2_GetActorLocation`)) (.y (`self.K2_GetActorLocation`)) (+ (.z (`self.K2_GetActorLocation`)) 50.0))) "AlwaysSpawn" "OverrideRootScale" null null))
  (`/Game/UniversalHealthSystem/Blueprints/Items/BP_Items_Master.-RandomStatCount` _returnvalue)
  (add `self.OnDestroyed` _returnvalue (`|CreateDelegate` :!event `-RespawnStart`))
  (set `self.Spawned` true))

(fn `-SpawnTimer`
  (bind _output_get (set `self.Timer` (- (`self.Timer`) 1)))
  (set `self.Name` (`KismetTextLibrary.Conv_IntToText` _output_get false false))
  (if (== _output_get 0)
    (bind _output_get_2 (set `self.Timer` (`self.SpawnTime`)))
    (set `self.Name` (`KismetTextLibrary.Conv_IntToText` _output_get_2 false false))
    (`self.-HiddenText_Server` true)
    (`KismetSystemLibrary.K2_ClearAndInvalidateTimerHandle` (`self.Timer-SpawnTimer`))
    (`self.-SpawnItem`)
    (else
      (`self.-HiddenText_Server` false))))

(fn `-StartTimerToRespawnItem`
  (`self.-HiddenText_Server` false)
  (bind _returnvalue (`KismetSystemLibrary.K2_SetTimer` null "-SpawnTimer" 1.0 true))
  (set `self.Timer-SpawnTimer` _returnvalue))

(fn `OnRep_Name`
  (`TextRenderComponent.K2_SetText` (`self.TextRender`) (`self.Name`))
  (if (== (`self.Timer`) 0)
    (`self.-HiddenText_Server` true)))

(fn `UserConstructionScript`)