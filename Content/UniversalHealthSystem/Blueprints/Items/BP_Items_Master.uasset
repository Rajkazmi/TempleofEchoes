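; Master pickup item for the health system that applies a stat change for HP, MP, Hunger or Thirst.
; Construction sets the text label from the stat type, and Tick turns it toward the camera while spinning the actor.
; Sphere overlap by a player-controlled actor calls a server-named event, which updates the pawn's BP_Stats_Component by Count and destroys the item.
; A separate event can randomize Count.
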(event `self.ReceiveTick`
  (params (DeltaSeconds :type "Float (single-precision)"))
  (bind _returnvalue (`GameplayStatics.GetPlayerCameraManager` 0))
  ;[1 1 1] Rotation to Camera and actor
  (`/Engine/EditorBlueprintResources/StandardMacros.IsValid` _returnvalue
    (:`Is Valid`
      (`SceneComponent.K2_SetWorldRotation` (`self.TextRender`) (`KismetMathLibrary.MakeRotator` 0.0 0.0 (+ (.yaw (`KismetMathLibrary.FindLookAtRotation` (`self.K2_GetActorLocation` _returnvalue) (`self.K2_GetActorLocation`))) 180.0)) false false)
      (`self.K2_AddActorWorldRotation` (struct :`Yaw` 0.5)))))

(event `self.Sphere.OnComponentBeginOverlap`
  (params (OverlappedComponent :type "PrimitiveComponent Object Reference") (OtherActor :type "Actor Object Reference") (OtherComp :type "PrimitiveComponent Object Reference") (OtherBodyIndex :type Integer) (bFromSweep :type Boolean) (SweepResult :type "HitResult Structure (by ref)"))
  (bind _returnvalue (`self.GetInstigatorController` OtherActor))
  (`/Engine/EditorBlueprintResources/StandardMacros.IsValid` OtherActor
    (:`Is Valid`
      (`/Engine/EditorBlueprintResources/StandardMacros.IsValid` _returnvalue
        (:`Is Valid`
          (bind _asplayer_controller (cast `PlayerController` _returnvalue))
          (`self.-ApplyItem-Server` _asplayer_controller))))))

(event `-ApplyItem-Server`
  (params (TargetPlayerController :type "PlayerController Object Reference"))
  (bind _returnvalue (`self.GetComponentByClass` (`Controller.K2_GetPawn` TargetPlayerController) "/Game/UniversalHealthSystem/Blueprints/Components/BP_Stats_Component.BP_Stats_Component_C"))
  ;[1 1 1] Apply Item
  (`/Engine/EditorBlueprintResources/StandardMacros.IsValid` _returnvalue
    (:`Is Valid`
      (`/Game/UniversalHealthSystem/Blueprints/Components/BP_Stats_Component.-UpdateTargetStat` _returnvalue (`self.Type`) (`KismetMathLibrary.Conv_IntToDouble` (`self.Count`)))
      (`self.K2_DestroyActor`))))

(event `-RandomStatCount`
  (set `self.Count` (`KismetMathLibrary.RandomIntegerInRange` 10 50)))

(fn `UserConstructionScript`
  (`TextRenderComponent.K2_SetText` (`self.TextRender`) (select `/Game/UniversalHealthSystem/Blueprints/Enums/E_Stats` (`self.Type`) :`NewEnumerator0` (`|FormatText` "Health Potion") :`NewEnumerator1` (`|FormatText` "Mana Potion") :`NewEnumerator2` (`|FormatText` "Energy Potion") :`NewEnumerator3` (`|FormatText` "Water Bottle"))))