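; Actor component that gives pawns replicated health, mana, hunger and thirst, with death and depletion dispatchers.
; Looping timers regenerate mana and drain hunger and thirst, which damage health at zero.
; Clamped update events change stats, while OnRep functions refresh the stats widget.
; Components register in the first player pawn's actor list, which optionally saves to a slot on controller EndPlay and reloads by name on init.
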(event `-InitOwner`
  (bind _returnvalue (`self.GetOwner`))
  ;[1 1 1] Init
  (bind _aspawn (cast `Pawn` (`self.GetOwner`)))
  (bind _output_get (set `self.Controller` (`Pawn.GetController` _aspawn)))
  (add `Actor.OnEndPlay` _output_get (`|CreateDelegate` :!event `-EndGame`))
  (`|ExecutionSequence`
    (:`then_0`
      (`self.-JoinNewPlayer` _returnvalue (`KismetTextLibrary.Conv_TextToString` (`KismetTextLibrary.Conv_StringToText` (`KismetSystemLibrary.GetObjectName` _returnvalue)))))
    (:`then_1`
      (`KismetSystemLibrary.Delay` (select `bool` (`KismetSystemLibrary.IsStandalone`) :`false` 1.5 :`true` 0.1))
      (`self.-UpdateStatsWidget`)
      (`|ExecutionSequence`
        (:`then_0`
          (if (`self.Hunger`)
            (bind _returnvalue_2 (`KismetSystemLibrary.K2_SetTimer` null "-RegenerationHunger" (`self.HungerTimerForPoint`) true))
            (set `self.Timer-RegenerationHunger` _returnvalue_2)))
        (:`then_1`
          (if (`self.Thirst`)
            (bind _returnvalue_3 (`KismetSystemLibrary.K2_SetTimer` null "-RegenerationThirst" (`self.ThirstTimerForPoint`) true))
            (set `self.Timer-RegenerationThirst` _returnvalue_3)))
        (:`then_2`
          (if (and (`self.RegenerationMP?`) (!= (`self.MaxMP`) (`self.CurrentMP`)))
            (bind _returnvalue_4 (`KismetSystemLibrary.K2_SetTimer` null "-RegenerationMP" (`self.SpeedRegenerationMP_InSeconds`) true))
            (set `self.Timer-RegenerationMP` _returnvalue_4)))))))

(event `-UpdateHealth`
  (params (Health :type "Float (double-precision)"))
  ;[1 1 1] Update Health
  (bind _output_get (set `self.CurrentHealth` (`KismetMathLibrary.FClamp` (+ Health (`self.CurrentHealth`)) 0.0 (`self.MaxHealth`))))
  (if (== _output_get 0.0)
    (set `self.IsDead` true)
    (`KismetSystemLibrary.K2_ClearAndInvalidateTimerHandle` (`self.Timer-RegenerationMP`))
    (`KismetSystemLibrary.K2_ClearAndInvalidateTimerHandle` (`self.Timer-RegenerationThirst`))
    (`KismetSystemLibrary.K2_ClearAndInvalidateTimerHandle` (`self.Timer-RegenerationHunger`))
    (`self.-CallIsDeadDisp-Multi`)))

(event `-CallIsDeadDisp-Multi`
  ;[1 1 1] Update Health
  (`self.IsDeadDispatcher`))

(event `-EndGame`
  (params (Actor :type "Actor Object Reference") (EndPlayReason :type "EEndPlayReason Enum" :default "Destroyed"))
  ;[1 1 1] End Game Bind Event
  (if (`self.SaveGame?`)
    (`self.-SaveStats`)))

(event `-UpdateMP`
  (params (ManaPoints :type "Float (double-precision)"))
  ;[1 1 1] Update MP
  (bind _output_get (set `self.CurrentMP` (`KismetMathLibrary.FClamp` (+ ManaPoints (`self.CurrentMP`)) 0.0 (`self.MaxMP`))))
  (if (< _output_get (`self.MaxMP`))
    (if (and (not (`KismetSystemLibrary.K2_IsTimerActiveHandle` (`self.Timer-RegenerationMP`))) (not (`self.IsDead`)) (`self.RegenerationMP?`))
      (bind _returnvalue (`KismetSystemLibrary.K2_SetTimer` null "-RegenerationMP" (`self.SpeedRegenerationMP_InSeconds`) true))
      (set `self.Timer-RegenerationMP` _returnvalue))
    (else
      (`KismetSystemLibrary.K2_ClearAndInvalidateTimerHandle` (`self.Timer-RegenerationMP`)))))

(event `-JoinNewPlayer`
  (params (Actor :type "Actor Object Reference") (Name :type String))
  (bind _actorsforsave (`/Game/UniversalHealthSystem/Blueprints/Components/BP_Stats_Component.ActorsForSave` (`Actor.GetComponentByClass` (`GameplayStatics.GetPlayerPawn` 0) "BP_Stats_Component_C")))
  ;[1 1 1] Join New Player
  (`KismetArrayLibrary.Array_AddUnique` _actorsforsave (make `/Game/UniversalHealthSystem/Blueprints/Str/Str_ActorsSaveInfo` Actor Name))
  (for _array_element _actorsforsave
    (`self.-RefreshActors` (`Actor.GetComponentByClass` (`.ActorRef_4_33B541D24CAEA77B6A6D20AE44B65A1F` (break `/Game/UniversalHealthSystem/Blueprints/Str/Str_ActorsSaveInfo` _array_element)) "BP_Stats_Component_C") _actorsforsave)))

(event `-UpdateStatsWidget`
  ;[1 1 1] Update Widget
  (bind _playerstatswidget (`self.PlayerStatsWidget`)
    (:`then`
      (if (not (`Widget.IsVisible` _playerstatswidget))
        (`Widget.SetVisibility` _playerstatswidget "Visible"))
      (`/Game/UniversalHealthSystem/Blueprints/UI/W_PlayerStats_Widget.-UpdateWidget` _playerstatswidget))
    (:`else`)))

(event `-RefreshActors`
  (params (PlayerControllers :type "Array of /Game/UniversalHealthSystem/Blueprints/Str/Str_ActorsSaveInfo Structure"))
  ;[1 1 1] Join New Player
  (bind _output_get (set `self.ActorsForSave` PlayerControllers))
  (for _array_element _output_get
    (bind (_actorref _name) (break `/Game/UniversalHealthSystem/Blueprints/Str/Str_ActorsSaveInfo` _array_element))
    (set `/Game/UniversalHealthSystem/Blueprints/Components/BP_Stats_Component.SaveName` _name (`Actor.GetComponentByClass` _actorref "BP_Stats_Component_C"))))

(event `-UpdateHunger`
  (params (HungerPoints :type "Float (double-precision)"))
  ;[1 1 1] Update Hunger
  (bind _output_get (set `self.CurrentHunger` (`KismetMathLibrary.FClamp` (+ HungerPoints (`self.CurrentHunger`)) 0.0 (`self.MaxHunger`))))
  (if (<= _output_get 0.0)
    (set `self.HungerIsOver` true)
    (`self.-UpdateHealth` (/ (`self.HungerTimerForPoint`) (/ -1.0 (`self.DamageHungerPerSecond`))))
    (`/Engine/EditorBlueprintResources/StandardMacros.DoOnce` false :!label _label
      (:`Completed`
        (`self.HungerIsOverDispatcher`)))
    (else
      (set `self.HungerIsOver` false)
      (goto _label :!via `Reset`))))

(event `-SaveStats`
  (bind _returnvalue (`self.GetOwner`))
  (bind _returnvalue_2 (`Actor.GetComponentByClass` _returnvalue "BP_Stats_Component_C"))
  ;[1 1 1] Save and Load
  (if (`KismetSystemLibrary.IsStandalone`)
    (`/Engine/EditorBlueprintResources/StandardMacros.IsValid` _returnvalue_2 :!label _label_2
      (:`Is Valid`
        (bind _returnvalue_3 (`GameplayStatics.CreateSaveGameObject` "/Game/UniversalHealthSystem/Blueprints/BP_SaveGame.BP_SaveGame_C"))
        (for (_array_element _array_index) (`/Game/UniversalHealthSystem/Blueprints/Components/BP_Stats_Component.ActorsForSave` _returnvalue_2)
          (bind _returnvalue_4 (`Actor.GetComponentByClass` (`.ActorRef_4_33B541D24CAEA77B6A6D20AE44B65A1F` (break `/Game/UniversalHealthSystem/Blueprints/Str/Str_ActorsSaveInfo` _array_element)) "BP_Stats_Component_C"))
          (`KismetArrayLibrary.Array_Set` (`/Game/UniversalHealthSystem/Blueprints/BP_SaveGame.SaveInfo` _returnvalue_3) _array_index (make `/Game/UniversalHealthSystem/Blueprints/Str/Str_SaveInfo` (`/Game/UniversalHealthSystem/Blueprints/Components/BP_Stats_Component.SaveName` _returnvalue_4) (`/Game/UniversalHealthSystem/Blueprints/Components/BP_Stats_Component.CurrentHealth` _returnvalue_4) (`/Game/UniversalHealthSystem/Blueprints/Components/BP_Stats_Component.CurrentMP` _returnvalue_4) (`/Game/UniversalHealthSystem/Blueprints/Components/BP_Stats_Component.CurrentHunger` _returnvalue_4) (`/Game/UniversalHealthSystem/Blueprints/Components/BP_Stats_Component.CurrentThirst` _returnvalue_4)) true))
        (`GameplayStatics.SaveGameToSlot` _returnvalue_3 "Stats")))
    (elif (== (`GameplayStatics.GetPlayerPawn` 0) _returnvalue)
      (goto _label_2))))

(event `-UpdateThirst`
  (params (ThirstPoints :type "Float (double-precision)"))
  ;[1 1 1] Update Thirst
  (bind _output_get (set `self.CurrentThirst` (`KismetMathLibrary.FClamp` (+ ThirstPoints (`self.CurrentThirst`)) 0.0 (`self.MaxThirst`))))
  (if (<= _output_get 0.0)
    (set `self.ThirstIsOver` true)
    (`self.-UpdateHealth` (/ (`self.ThirstTimerForPoint`) (/ -1.0 (`self.DamageThirstPerSecond`))))
    (`/Engine/EditorBlueprintResources/StandardMacros.DoOnce` false :!label _label_3
      (:`Completed`
        (`self.ThirstIsOverDispatcher`)))
    (else
      (set `self.ThirstIsOver` false)
      (goto _label_3 :!via `Reset`))))

(event `-LoadStats`
  ;[1 1 1] Save and Load
  (bind _returnvalue (`GameplayStatics.LoadGameFromSlot` "Stats"))
  (bind _asbp_save_game (cast `/Game/UniversalHealthSystem/Blueprints/BP_SaveGame` _returnvalue))
  (for _array_element (`/Game/UniversalHealthSystem/Blueprints/BP_SaveGame.SaveInfo` _asbp_save_game)
    (bind (_name _health _mana _hunger _thirst) (break `/Game/UniversalHealthSystem/Blueprints/Str/Str_SaveInfo` _array_element))
    (if (`KismetStringLibrary.EqualEqual_StrStr` _name (`self.SaveName`))
      (set `self.CurrentHealth` _health)
      (set `self.CurrentMP` _mana)
      (set `self.CurrentHunger` _hunger)
      (set `self.CurrentThirst` _thirst)
      (break))))

(event `-UpdateTargetStat`
  (params (Stats :type "/Game/UniversalHealthSystem/Blueprints/Enums/E_Stats Enum" :default "NewEnumerator0") (Count :type "Float (double-precision)"))
  ;[1 1 1] Update Target Stat
  (switch `/Game/UniversalHealthSystem/Blueprints/Enums/E_Stats` Stats
    (:`NewEnumerator0`
      (`self.-UpdateHealth` Count))
    (:`NewEnumerator1`
      (`self.-UpdateMP` Count))
    (:`NewEnumerator2`
      (`self.-UpdateHunger` Count))
    (:`NewEnumerator3`
      (`self.-UpdateThirst` Count))))

(fn `-Init`
  (`self.-InitOwner`)
  (if (`self.LoadGame?`)
    (`self.-LoadStats`)
    (if (== (`self.CurrentHealth`) 0.0)
      (set `self.CurrentHealth` (`self.MaxHealth`) :!label _label)
      (set `self.CurrentMP` (`self.MaxMP`))
      (set `self.CurrentHunger` (`self.MaxHunger`))
      (set `self.CurrentThirst` (`self.MaxThirst`)))
    (else
      (goto _label)))
  (`self.-UpdateHealth` 0.0))

(fn `-RegenerationHunger`
  (`self.-UpdateHunger` -1.0))

(fn `-RegenerationMP`
  (`self.-UpdateMP` 1.0))

(fn `-RegenerationThirst`
  (`self.-UpdateThirst` -1.0))

(fn `OnRep_CurrentHealth`
  (`self.-UpdateStatsWidget`))

(fn `OnRep_CurrentHunger`
  (`self.-UpdateStatsWidget`))

(fn `OnRep_CurrentMP`
  (`self.-UpdateStatsWidget`))

(fn `OnRep_CurrentThirst`
  (`self.-UpdateStatsWidget`))