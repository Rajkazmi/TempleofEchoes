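; BP_Fireball is a fireball actor in the Universal Health System that damages what it overlaps and then explodes.
; Its Sphere overlap ignores the instigator, applies Damage to any other actor with the instigator as damage causer, then calls Boom.
; BeginPlay also calls Boom after DelayToDestroy, so the fireball expires on its own.
; Boom spawns the P_Explosion emitter at the actor's location and destroys the actor.
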(event `self.ReceiveBeginPlay`
  (`KismetSystemLibrary.Delay` (`self.DelayToDestroy`))
  (`self.-Boom`))

(event `-Boom`
  (`GameplayStatics.SpawnEmitterAtLocation` "/Game/UniversalHealthSystem/DemoContent/StarterContent/Particles/P_Explosion.P_Explosion" (`self.K2_GetActorLocation`))
  (`self.K2_DestroyActor`))

(event `self.Sphere.OnComponentBeginOverlap`
  (params (OverlappedComponent :type "PrimitiveComponent Object Reference") (OtherActor :type "Actor Object Reference") (OtherComp :type "PrimitiveComponent Object Reference") (OtherBodyIndex :type Integer) (bFromSweep :type Boolean) (SweepResult :type "HitResult Structure (by ref)"))
  (bind _returnvalue (`self.GetInstigator`))
  (if (!= OtherActor _returnvalue)
    (`GameplayStatics.ApplyDamage` OtherActor (`self.Damage`) null _returnvalue)
    (`self.-Boom`)))

(fn `UserConstructionScript`)